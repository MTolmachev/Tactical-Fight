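; BP_Pawn is a player camera pawn that pans, turns and zooms on a spring arm.
; Axis inputs adjust a desired location along the actor's forward and right vectors and a clamped desired arm length, while action presses step the desired yaw.
; Tick smoothly interpolates the arm length, location and rotation toward those targets, moving without sweep.
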(event EventTick
  (params (DeltaSeconds :type Float%20%28single-precision%29))
  (bind _springarm (Variables|Default|GetSpringArm))
  (Variables|/Script/Engine.SpringArmComponent|SetTargetArmLength _springarm (Math|Interpolation|FInterpTo (Variables|/Script/Engine.SpringArmComponent|GetTargetArmLength _springarm) (Variables|Zoom|GetZoom_Desired) (Utilities|Time|GetWorldDeltaSeconds) (Variables|Zoom|GetZoom_Interp)))
  (Transformation|SetActorLocation (Math|Interpolation|VInterpTo (Transformation|GetActorLocation) (Variables|Location|GetLocation_Desired) (Utilities|Time|GetWorldDeltaSeconds) (Variables|Location|GetLocation_Interp)) false false)
  (Transformation|SetActorRotation (Math|Interpolation|RInterpTo (Transformation|GetActorRotation) (Variables|Rotation|GetRotation_Desired) (Utilities|Time|GetWorldDeltaSeconds) (Variables|Rotation|GetRotation_Interp))))

(event EventBeginPlay
  (Variables|Zoom|SetZoom_Desired (Variables|/Script/Engine.SpringArmComponent|GetTargetArmLength (Variables|Default|GetSpringArm)))
  (Variables|Location|SetLocation_Desired (Transformation|GetActorLocation))
  (Variables|Rotation|SetRotation_Desired (Transformation|GetActorRotation)))

(event Input|ActionEvents|InputActionInputAction_RotationRight
  (params (Key :type Key%20Structure :default "None"))
  (:Pressed
    (Variables|Rotation|SetRotation_Desired (Math|Rotator|CombineRotators (Variables|Rotation|GetRotation_Desired) (Math|Rotator|MakeRotator 0.0 0.0 (* (Variables|Rotation|GetRotation_Speed) -1.0))))))

(event Input|ActionEvents|InputActionInputAction_RotationLeft
  (params (Key :type Key%20Structure :default "None"))
  (:Pressed
    (Variables|Rotation|SetRotation_Desired (Math|Rotator|CombineRotators (Variables|Rotation|GetRotation_Desired) (Math|Rotator|MakeRotator 0.0 0.0 (Variables|Rotation|GetRotation_Speed))))))

(event Input|AxisEvents|InputAxisInputAxis_Zoom
  (params (AxisValue :type Float%20%28single-precision%29))
  (Variables|Zoom|SetZoom_Desired (Math|Float|Clamp(Float) (+ (Variables|Zoom|GetZoom_Desired) (* AxisValue (Variables|Zoom|GetZoom_Speed))) (Variables|Zoom|GetZoom_Min) (Variables|Zoom|GetZoom_Max))))

(event Input|AxisEvents|InputAxisInputAxis_Forward
  (params (AxisValue :type Float%20%28single-precision%29))
  (Variables|Location|SetLocation_Desired (+ (Variables|Location|GetLocation_Desired) (* (* AxisValue (Variables|Location|GetLocation_Speed)) (Transformation|GetActorForwardVector)))))

(event Input|AxisEvents|InputAxisInputAxis_Right
  (params (AxisValue :type Float%20%28single-precision%29))
  (Variables|Location|SetLocation_Desired (+ (Variables|Location|GetLocation_Desired) (* (* AxisValue (Variables|Location|GetLocation_Speed)) (Transformation|GetActorRightVector)))))

(fn ConstructionScript)