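; Spell animation actor that shows a wind gust moving between two transforms.
; On BeginPlay, a timeline at a configurable play rate lerps the actor from its origin to its target transform and drives the gust material's Opacity parameter.
; When the timeline finishes, it fires the shape-animation-completed dispatcher, then destroys itself after a short delay.
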(event EventBeginPlay
  (Components|Timeline|SetPlayRate (Variables|Default|GetTimeline) (Variables|Default|GetPlayRate))
  (bind (_direction _transformalpha _opacity) (Timeline|Timeline PlayFromStart)
    (:Update
      (Transformation|SetActorTransform (Math|Transform|Lerp(Transform) (Variables|Default|GetOriginTransform) (Variables|Default|GetTargetTransform) _transformalpha))
      (Rendering|Material|SetScalarParameterValueonMaterials (Variables|Default|GetAnimatedWindGust) "Opacity" _opacity))
    (:Finished
      (Default|CallOnShapeAnimationCompleted self)
      (Utilities|FlowControl|Delay 1.0)
      (Actor|DestroyActor))))

(fn ConstructionScript)