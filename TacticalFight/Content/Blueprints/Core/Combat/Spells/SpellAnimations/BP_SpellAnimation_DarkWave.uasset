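; BP_SpellAnimation_DarkWave is a spell animation actor that plays the Dark Wave visual effect on a target tile during combat.
; When triggered, it moves to the target tile's location and runs a timeline that scales the AnimScale component and drives an Opacity material parameter on three static meshes.
; When the timeline finishes, it signals that the spell animation is complete.
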(event EventBeginPlay
  (|CallParentFunction) ; This node is disabled and will not be called.\nDrag off pins to build functionality.
)

(event Collision|EventActorBeginOverlap
  (params (OtherActor :type Actor%20Object%20Reference)))

(event EventTick
  (params (DeltaSeconds :type Float%20%28single-precision%29)))

(event EventEventPlaySpellAnimation
  (Transformation|SetActorLocation (.location (CallFunction|GetTileTransform (Variables|Default|GetTargetIndex))) false false)
  (bind (_direction _opacity _scale) (Timeline|Timeline_DarkWave Play)
    (:Update
      (Transformation|SetRelativeScale3D (Variables|Default|GetAnim_Scale) _scale)
      (Rendering|Material|SetScalarParameterValueonMaterials (Variables|Default|GetStaticMesh1) "Opacity" _opacity))
    (:Finished
      (CallFunction|EventCompleteSpellAnimation))))

(fn ConstructionScript
  (|CallParentFunction))