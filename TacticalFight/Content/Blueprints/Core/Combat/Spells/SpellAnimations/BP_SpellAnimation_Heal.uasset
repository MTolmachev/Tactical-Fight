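; Spell animation actor that plays the visual effect for a heal spell on a target tile.
; On the play event it moves to the target tile's transform and runs a timeline that scales and yaw-rotates a pivot component while driving Opacity on six mesh materials, including plus-sign meshes.
; When the timeline finishes, it fires the completion event to end the spell animation.
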(event EventBeginPlay
  (|CallParentFunction) ; This node is disabled and will not be called.\nDrag off pins to build functionality.
)

(event Collision|EventActorBeginOverlap
  (params (OtherActor :type Actor%20Object%20Reference)))

(event EventTick
  (params (DeltaSeconds :type Float%20%28single-precision%29)))

(event EventEventPlaySpellAnimation
  (bind _anim_rotationscale (Variables|Default|GetAnim_RotationScale))
  (Transformation|SetActorLocation (.location (CallFunction|GetTileTransform (Variables|Default|GetTargetIndex))) false false)
  (bind (_direction _opacity _scale _rotation) (Timeline|Timeline_Heal Play)
    (:Update
      (Transformation|SetRelativeScale3D _anim_rotationscale _scale)
      (Transformation|SetRelativeRotation _anim_rotationscale (Math|Rotator|MakeRotator 0.0 0.0 _rotation) false false)
      (Rendering|Material|SetScalarParameterValueonMaterials (Variables|Default|GetStaticMesh1) "Opacity" _opacity))
    (:Finished
      (CallFunction|EventCompleteSpellAnimation))))

(fn ConstructionScript
  (|CallParentFunction))