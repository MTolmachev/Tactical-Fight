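; Spell animation actor for the Slime Ball combat spell, which sends a slime ball from the origin tile to the target tile.
; On play, it snaps to the origin tile, then a timeline lerps its location between tiles with an added height offset curve.
; The same timeline drives the opacity material parameter on three meshes and the scale of the AnimScale component.
; When the timeline finishes, it signals that the spell animation is complete.
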(event EventBeginPlay
  (|CallParentFunction) ; This node is disabled and will not be called.\nDrag off pins to build functionality.
)

(event Collision|EventActorBeginOverlap
  (params (OtherActor :type Actor%20Object%20Reference)))

(event EventTick
  (params (DeltaSeconds :type Float%20%28single-precision%29)))

(event EventEventPlaySpellAnimation
  (Transformation|SetActorLocation (.location (CallFunction|GetTileTransform (Variables|Default|GetOriginIndex))) false false)
  (bind (_direction _locationalpha _locationz _opacity _scale) (Timeline|Timeline_SlimeBall PlayFromStart)
    (:Update
      (Transformation|SetActorLocation (+ (Math|Vector|Lerp(Vector) (.location (CallFunction|GetTileTransform (Variables|Default|GetOriginIndex))) (.location (CallFunction|GetTileTransform (Variables|Default|GetTargetIndex))) _locationalpha) (Math|Vector|MakeVector 0.0 0.0 _locationz)) false false)
      (Rendering|Material|SetScalarParameterValueonMaterials (Variables|Default|GetStaticMesh) "Opacity" _opacity)
      (Transformation|SetRelativeScale3D (Variables|Default|GetAnim_Scale) _scale))
    (:Finished
      (CallFunction|EventCompleteSpellAnimation))))

(fn ConstructionScript
  (|CallParentFunction))